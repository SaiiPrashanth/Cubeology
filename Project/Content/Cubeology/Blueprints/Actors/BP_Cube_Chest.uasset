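; Chest variant of a cube actor that opens and closes its lid when interacted with.
; On BeginPlay, after the parent logic, the chest top copies the first material of the block mesh so the two match.
; Each Interact alternates through a FlipFlop between playing and reversing a timeline, whose value drives the relative pitch of the ChestOpener component.
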(event EventBeginPlay
  (|CallParentFunction)
  (Rendering|Material|SetMaterial (Variables|Default|GetSM_Chest_Top) 0 (Rendering|Material|GetMaterial (Variables|Default|GetSM_Block) 0)))

(event EventInteract
  (Utilities|FlowControl|FlipFlop
    (:A
      (bind _chestopen (Timeline|ChestOpenTimeline Play)
        (:Update
          (Transformation|SetRelativeRotation (Variables|Default|GetChestOpener) (Math|Rotator|MakeRotator 0.0 _chestopen 0.0) false false))))
    (:B
      (Timeline|ChestOpenTimeline Reverse))))

(fn ConstructionScript
  (|CallParentFunction))