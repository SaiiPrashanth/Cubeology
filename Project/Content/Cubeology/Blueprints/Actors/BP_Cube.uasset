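; BP_Cube is a block actor in Cubeology that can be destroyed over time, with the option to cancel.
; On BeginPlay it creates a dynamic material instance on the SMBlock mesh and sets the timeline play rate from DestroyRate.
; StartDestroyCube plays a timeline that drives the DestroySlider material parameter, destroying the actor when finished.
; StopDestroyCube resets the parameter and stops the timeline.
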(event Custom|StopDestroyCube
  (Rendering|Material|SetScalarParameterValue (Variables|Default|GetCubeMatInst) "DestroySlider" 0.0 :!class /Script/Engine.MaterialInstanceDynamic)
  (bind _destroycube (Timeline|DestroyTimeline Stop)
    (:Update
      (Rendering|Material|SetScalarParameterValue (Variables|Default|GetCubeMatInst) "DestroySlider" _destroycube :!class /Script/Engine.MaterialInstanceDynamic))
    (:Finished
      (Actor|DestroyActor))))

(event Custom|StartDestroyCube
  (bind _destroycube (Timeline|DestroyTimeline PlayFromStart)
    (:Update
      (Rendering|Material|SetScalarParameterValue (Variables|Default|GetCubeMatInst) "DestroySlider" _destroycube :!class /Script/Engine.MaterialInstanceDynamic))
    (:Finished
      (Actor|DestroyActor))))

(event EventBeginPlay
  (bind _sm_block (Variables|Default|GetSM_Block))
  (bind _returnvalue (Rendering|Material|CreateDynamicMaterialInstance _sm_block 0 (Rendering|Material|GetMaterial _sm_block 0) "None" :!class /Script/Engine.PrimitiveComponent))
  (Variables|Default|SetCubeMatInst _returnvalue)
  (Components|Timeline|SetPlayRate (Variables|Default|GetDestroyTimeline) (Variables|Default|GetDestroyRate)))

(fn ConstructionScript)