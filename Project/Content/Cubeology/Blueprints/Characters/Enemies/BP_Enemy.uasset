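; BP_Enemy is an enemy character that chases and attacks the player once it sees a pawn.
; PawnSensing sets a seeing flag and calls FollowPlayer, which runs AI MoveTo targeting the player controller, not its pawn.
; On arrival it plays the AM_Manny montage, with CanAttack and a montage-length delay blocking overlapping attacks.
; The seeing flag is never cleared here, and no damage is applied in this graph.
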(event OnSeePawn(PawnSensing)
  (params (Pawn :type Pawn%20Object%20Reference))
  (Variables|Default|SetisSeeingPlayer? true)
  (CallFunction|FollowPlayer))

(event Custom|FollowPlayer
  (if (Variables|Default|GetisSeeingPlayer?)
    (AI|AIMoveTo self "0, 0, 0" (Game|GetPlayerController 0) 7e+01 false
      (:OnSuccess
        (if (Variables|Default|GetCanAttack?)
          (Variables|Default|SetCanAttack? false)
          (bind _returnvalue (Animation|PlayAnimMontage "/Game/AM_Manny.AM_Manny" 1.0 "None"))
          (Utilities|FlowControl|Delay _returnvalue)
          (Variables|Default|SetCanAttack? true))))))

(fn ConstructionScript)